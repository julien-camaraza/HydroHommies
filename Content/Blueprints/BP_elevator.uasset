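; Elevator actor that moves its Cube component from its starting position to the position of GoToLocation.
; BeginPlay caches both world positions, sets the Moving timeline's play rate from Speed and starts it immediately, with no trigger.
; Each timeline update lerps the Cube's world location by the MovementFloat track, without sweeping for collisions.
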(event `self.ReceiveBeginPlay`
  (set `self.startingLocation` (`SceneComponent.K2_GetComponentLocation` (`self.Cube`)))
  (set `self.endingLocation` (`SceneComponent.K2_GetComponentLocation` (`self.goToLocation`)))
  (`TimelineComponent.SetPlayRate` (`self.moving`) (`self.Speed`))
  (bind (_direction _movementfloat) (`Timeline|moving` :!via `PlayFromStart`)
    (:`Update`
      (`SceneComponent.K2_SetWorldLocation` (`self.Cube`) (`KismetMathLibrary.VLerp` (`self.startingLocation`) (`self.endingLocation`) _movementfloat) false false))))

(fn `UserConstructionScript`)