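; Ice wall actor that rises to a given size, holds for a while, then sinks away and destroys itself.
; The createWall event takes a scale vector, enlarges it by a fixed factor and drives three chained timelines: Grow, Wait and Die.
; Grow and Die lerp only the IceWall component's Z scale between zero and full height, while Wait serves purely as a delay.
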(event `createWall`
  (params (A :type "Vector Structure"))
  (bind _returnvalue (* A 1.2))
  (bind _returnvalue_2 (`KismetMathLibrary.MakeVector` (.x _returnvalue) (.y _returnvalue)))
  (bind _returnvalue_3 (`KismetMathLibrary.MakeVector` (.x _returnvalue) (.y _returnvalue) (.z _returnvalue)))
  (bind (_direction _newtrack_0) (`Timeline|grow` :!via `PlayFromStart`)
    (:`Update`
      (`SceneComponent.SetWorldScale3D` (`self.iceWall`) (`KismetMathLibrary.VLerp` _returnvalue_2 _returnvalue_3 _newtrack_0)))
    (:`Finished`
      (`Timeline|wait` :!via `PlayFromStart`
        (:`Finished`
          (bind (_direction_2 _newtrack_0_2) (`Timeline|die` :!via `PlayFromStart`)
            (:`Update`
              (`SceneComponent.SetWorldScale3D` (`self.iceWall`) (`KismetMathLibrary.VLerp` _returnvalue_3 _returnvalue_2 _newtrack_0_2)))
            (:`Finished`
              (`self.K2_DestroyActor`))))))))

(fn `UserConstructionScript`)