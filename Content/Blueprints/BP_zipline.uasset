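; Zipline actor that lets BP_Multiplayer_Character know when it can ride the spline, and in which direction.
; Capsule overlaps with StartingBox or EndingBox pass the spline to the character, flag it as near, and set travel forwards or backwards respectively.
; Leaving StartingBox clears this unless the character is zipline-jumping.
; EndingBox's exit compares its own component to the capsule, so its matching clear appears unreachable.
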(event `self.startingBox.OnComponentBeginOverlap`
  (params (OverlappedComponent :type "PrimitiveComponent Object Reference") (OtherActor :type "Actor Object Reference") (OtherComp :type "PrimitiveComponent Object Reference") (OtherBodyIndex :type Integer) (bFromSweep :type Boolean) (SweepResult :type "HitResult Structure (by ref)"))
  (bind _asbp_multiplayer_character (cast `/Game/MultiplayerStarterPack/Blueprints/BP_Multiplayer_Character` OtherActor))
  (if (== OtherComp (`Character.CapsuleComponent` _asbp_multiplayer_character))
    (set `/Game/MultiplayerStarterPack/Blueprints/BP_Multiplayer_Character.ziplineForwards` true _asbp_multiplayer_character)
    (set `/Game/MultiplayerStarterPack/Blueprints/BP_Multiplayer_Character.ziplineSpline` (`self.Spline`) _asbp_multiplayer_character)
    (set `/Game/MultiplayerStarterPack/Blueprints/BP_Multiplayer_Character.nearZipline` true _asbp_multiplayer_character)
    (`KismetSystemLibrary.PrintString` "nearZipline")))

(event `self.startingBox.OnComponentEndOverlap`
  (params (OverlappedComponent :type "PrimitiveComponent Object Reference") (OtherActor :type "Actor Object Reference") (OtherComp :type "PrimitiveComponent Object Reference") (OtherBodyIndex :type Integer))
  (bind _asbp_multiplayer_character (cast `/Game/MultiplayerStarterPack/Blueprints/BP_Multiplayer_Character` OtherActor))
  (if (== OtherComp (`Character.CapsuleComponent` _asbp_multiplayer_character))
    (if (not (`/Game/MultiplayerStarterPack/Blueprints/BP_Multiplayer_Character.ziplineJumping` _asbp_multiplayer_character))
      (set `/Game/MultiplayerStarterPack/Blueprints/BP_Multiplayer_Character.ziplineSpline` null _asbp_multiplayer_character)
      (set `/Game/MultiplayerStarterPack/Blueprints/BP_Multiplayer_Character.nearZipline` false _asbp_multiplayer_character)
      (`KismetSystemLibrary.PrintString` "noZip"))))

(event `self.endingBox.OnComponentBeginOverlap`
  (params (OverlappedComponent :type "PrimitiveComponent Object Reference") (OtherActor :type "Actor Object Reference") (OtherComp :type "PrimitiveComponent Object Reference") (OtherBodyIndex :type Integer) (bFromSweep :type Boolean) (SweepResult :type "HitResult Structure (by ref)"))
  (bind _asbp_multiplayer_character (cast `/Game/MultiplayerStarterPack/Blueprints/BP_Multiplayer_Character` OtherActor))
  (if (== OtherComp (`Character.CapsuleComponent` _asbp_multiplayer_character))
    (set `/Game/MultiplayerStarterPack/Blueprints/BP_Multiplayer_Character.ziplineForwards` false _asbp_multiplayer_character)
    (set `/Game/MultiplayerStarterPack/Blueprints/BP_Multiplayer_Character.ziplineSpline` (`self.Spline`) _asbp_multiplayer_character)
    (set `/Game/MultiplayerStarterPack/Blueprints/BP_Multiplayer_Character.nearZipline` true _asbp_multiplayer_character)
    (`KismetSystemLibrary.PrintString` "nearZipline")))

(event `self.endingBox.OnComponentEndOverlap`
  (params (OverlappedComponent :type "PrimitiveComponent Object Reference") (OtherActor :type "Actor Object Reference") (OtherComp :type "PrimitiveComponent Object Reference") (OtherBodyIndex :type Integer))
  (bind _asbp_multiplayer_character (cast `/Game/MultiplayerStarterPack/Blueprints/BP_Multiplayer_Character` OtherActor))
  (if (== OverlappedComponent (`Character.CapsuleComponent` _asbp_multiplayer_character))
    (if (not (`/Game/MultiplayerStarterPack/Blueprints/BP_Multiplayer_Character.ziplineJumping` _asbp_multiplayer_character))
      (set `/Game/MultiplayerStarterPack/Blueprints/BP_Multiplayer_Character.ziplineSpline` null _asbp_multiplayer_character)
      (set `/Game/MultiplayerStarterPack/Blueprints/BP_Multiplayer_Character.nearZipline` false _asbp_multiplayer_character)
      (`KismetSystemLibrary.PrintString` "noZip"))))

(fn `UserConstructionScript`
  (`|ExecutionSequence`))