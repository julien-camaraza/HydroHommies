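; BP_smoke is a thrown or launched projectile that turns into a temporary expanding sphere, apparently a smoke cloud, on impact.
; On its first hit, Sphere1, which projectile movement drives, stops simulating physics and is hidden while Sphere2 is shown.
; Chained timelines scale Sphere2 from zero to SizeToBecome, hold it for the Wait timeline, shrink it back, then destroy the actor.
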(event `self.Sphere1.OnComponentHit`
  (params (HitComponent :type "PrimitiveComponent Object Reference") (OtherActor :type "Actor Object Reference") (OtherComp :type "PrimitiveComponent Object Reference") (NormalImpulse :type "Vector Structure") (Hit :type "HitResult Structure (by ref)"))
  (`/Engine/EditorBlueprintResources/StandardMacros.DoOnce` false
    (:`Completed`
      (`PrimitiveComponent.SetSimulatePhysics` (`self.Sphere1`) false)
      (`SceneComponent.SetVisibility` (`self.Sphere2`) true false)
      (`SceneComponent.SetVisibility` (`self.Sphere1`) false false)
      (bind (_direction _newtrack_0) (`Timeline|vfxGrowth` :!via `PlayFromStart`)
        (:`Update`
          (`SceneComponent.SetWorldScale3D` (`self.Sphere2`) (`KismetMathLibrary.VLerp` (0.0 0.0 0.0) (`self.sizeToBecome`) _newtrack_0)))
        (:`Finished`
          (`Timeline|wait`
            (:`Finished`
              (bind (_direction_2 _newtrack_0_2) (`Timeline|Timeline_0` :!via `ReverseFromEnd`)
                (:`Update`
                  (`SceneComponent.SetWorldScale3D` (`self.Sphere2`) (`KismetMathLibrary.VLerp` (0.0 0.0 0.0) (`self.sizeToBecome`) _newtrack_0_2)))
                (:`Finished`
                  (`self.K2_DestroyActor`))))))))))

(fn `UserConstructionScript`
  (`MovementComponent.SetUpdatedComponent` (`self.ProjectileMovement`) (`self.Sphere1`)))