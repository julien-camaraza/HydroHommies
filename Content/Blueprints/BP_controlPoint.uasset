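; Capturable team control point for multiplayer that tracks Red and Blue players on it and refills the water of characters inside its box.
; Overlap counts decide which team's looping timer runs, draining the rival's control before building its own, scaled by headcount advantage.
; Passing the capture threshold sets the owning team and tints the cone and beam dynamic materials.
; Stat changes are pushed through BP_MultiPlayerGameMode.
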(event `self.ReceiveTick`
  (params (DeltaSeconds :type "Float (single-precision)")))

(event `reset`
  (set `self.blueTeamControl` 0.0)
  (set `self.redTeamControl` 0.0)
  (set `self.numberOfRedOnPoint` 0)
  (set `self.numberOfBlueOnPoint` 0)
  (set `self.team` "NewEnumerator2")
  (`MaterialInstanceDynamic.SetVectorParameterValue` (`self.matInst`) "Color" (struct :`R` 0.859375 :`G` 0.859375 :`B` 0.859375 :`A` 1.0))
  (`MaterialInstanceDynamic.SetVectorParameterValue` (`self.matBeamLight`) "Color" (struct :`R` 0.859375 :`G` 0.859375 :`B` 0.859375 :`A` 1.0))
  (`self.clearTimers`))

(event `removeMe`
  (params (team :type "/Game/Blueprints/ENUM_teams Enum" :default "NewEnumerator2"))
  (switch `/Game/Blueprints/ENUM_teams` team
    (:`NewEnumerator0`
      (`/Engine/EditorBlueprintResources/StandardMacros.DecrementInt` (`self.numberOfRedOnPoint`)
        (:`  `
          _)))
    (:`NewEnumerator1`
      (`/Engine/EditorBlueprintResources/StandardMacros.DecrementInt` (`self.numberOfBlueOnPoint`)
        (:`  `
          _))))
  (`self.evaluateControl`))

(event `self.Box.OnComponentBeginOverlap`
  (params (OverlappedComponent :type "PrimitiveComponent Object Reference") (OtherActor :type "Actor Object Reference") (OtherComp :type "PrimitiveComponent Object Reference") (OtherBodyIndex :type Integer) (bFromSweep :type Boolean) (SweepResult :type "HitResult Structure (by ref)"))
  (bind _asbp_multiplayer_character (cast `/Game/MultiplayerStarterPack/Blueprints/BP_Multiplayer_Character` OtherActor))
  (if (== OtherComp (`Character.CapsuleComponent` _asbp_multiplayer_character))
    (bind _returnvalue (`KismetSystemLibrary.K2_SetTimerDelegate` (delegate `refillWater`) 0.1 true))))

(event `refillWater`
  (`/Engine/EditorBlueprintResources/StandardMacros.IsValid` (stale `self.Box.OnComponentBeginOverlap` _asbp_multiplayer_character)
    (:`Is Valid`
      (set `/Game/MultiplayerStarterPack/Blueprints/BP_Multiplayer_Character.waterRemaining` (`KismetMathLibrary.FClamp` (+ (`/Game/MultiplayerStarterPack/Blueprints/BP_Multiplayer_Character.waterRemaining` (stale `self.Box.OnComponentBeginOverlap` _asbp_multiplayer_character)) 1.0) 0.0 100.0) (stale `self.Box.OnComponentBeginOverlap` _asbp_multiplayer_character)))))

(event `self.ReceiveActorBeginOverlap`
  (params (OtherActor :type "Actor Object Reference"))
  (bind _asbp_multiplayer_character (cast `/Game/MultiplayerStarterPack/Blueprints/BP_Multiplayer_Character` OtherActor))
  (if (not (`/Game/MultiplayerStarterPack/Blueprints/BP_Multiplayer_Character.Dead` _asbp_multiplayer_character))
    (set `/Game/MultiplayerStarterPack/Blueprints/BP_Multiplayer_Character.controlPointStanding` self _asbp_multiplayer_character)
    (switch `/Game/Blueprints/ENUM_teams` (`/Game/MultiplayerStarterPack/Blueprints/BP_Multiplayer_Character.team` _asbp_multiplayer_character)
      (:`NewEnumerator0`
        (`/Engine/EditorBlueprintResources/StandardMacros.IncrementInt` (`self.numberOfRedOnPoint`)
          (:`  `
            (`/Engine/EditorBlueprintResources/StandardMacros.IncrementInt` (`self.numberOfRedOnPoint`)
              (:`  `
                _)))))
      (:`NewEnumerator1`
        (`/Engine/EditorBlueprintResources/StandardMacros.IncrementInt` (`self.numberOfBlueOnPoint`)
          (:`  `
            (`/Engine/EditorBlueprintResources/StandardMacros.IncrementInt` (`self.numberOfBlueOnPoint`)
              (:`  `
                _))))))
    (`self.evaluateControl` :!label _label)))

(event `self.Box.OnComponentEndOverlap`
  (params (OverlappedComponent :type "PrimitiveComponent Object Reference") (OtherActor :type "Actor Object Reference") (OtherComp :type "PrimitiveComponent Object Reference") (OtherBodyIndex :type Integer))
  (cast `/Game/MultiplayerStarterPack/Blueprints/BP_Multiplayer_Character` OtherActor)
  (`KismetSystemLibrary.K2_ClearAndInvalidateTimerHandle` (stale `self.Box.OnComponentBeginOverlap` _returnvalue)))

(event `self.ReceiveActorEndOverlap`
  (params (OtherActor :type "Actor Object Reference"))
  (bind _asbp_multiplayer_character (cast `/Game/MultiplayerStarterPack/Blueprints/BP_Multiplayer_Character` OtherActor))
  (set `/Game/MultiplayerStarterPack/Blueprints/BP_Multiplayer_Character.controlPointStanding` null _asbp_multiplayer_character)
  (switch `/Game/Blueprints/ENUM_teams` (`/Game/MultiplayerStarterPack/Blueprints/BP_Multiplayer_Character.team` _asbp_multiplayer_character)
    (:`NewEnumerator0`
      (`/Engine/EditorBlueprintResources/StandardMacros.DecrementInt` (`self.numberOfRedOnPoint`)
        (:`  `
          (`/Engine/EditorBlueprintResources/StandardMacros.DecrementInt` (`self.numberOfRedOnPoint`)
            (:`  `
              (goto _label))))))
    (:`NewEnumerator1`
      (`/Engine/EditorBlueprintResources/StandardMacros.DecrementInt` (`self.numberOfBlueOnPoint`)
        (:`  `
          (`/Engine/EditorBlueprintResources/StandardMacros.DecrementInt` (`self.numberOfBlueOnPoint`)
            (:`  `
              (goto _label))))))))

(event `evaluateControl`
  (if (or (> (`self.numberOfRedOnPoint`) 0) (> (`self.numberOfBlueOnPoint`) 0))
    (if (> (`self.numberOfRedOnPoint`) (`self.numberOfBlueOnPoint`))
      (bind _returnvalue (`KismetSystemLibrary.K2_SetTimerDelegate` (delegate `redControlling`) 1.0 true))
      (if (`KismetSystemLibrary.K2_IsValidTimerHandle` (stale _returnvalue_2)) :!label _label_2
        (`KismetSystemLibrary.K2_ClearAndInvalidateTimerHandle` (stale _returnvalue_2))
        (`self.updatePlayerStats`))
      (elif (> (`self.numberOfBlueOnPoint`) (`self.numberOfRedOnPoint`))
        (bind _returnvalue_2 (`KismetSystemLibrary.K2_SetTimerDelegate` (delegate `blueControlling`) 1.0 true))
        (if (`KismetSystemLibrary.K2_IsValidTimerHandle` _returnvalue) :!label _label_3
          (`KismetSystemLibrary.K2_ClearAndInvalidateTimerHandle` _returnvalue))))
    (else
      (`self.updatePlayerStats`))))

(event `pauseChecking`)

(event `redControlling`
  (bind _blueteamcontrol (`self.blueTeamControl`))
  (if (> _blueteamcontrol 0.0)
    (set `self.blueTeamControl` (`KismetMathLibrary.FClamp` (- _blueteamcontrol 1.0) 0.0 100.0))
    (else
      (set `self.team` "NewEnumerator2")
      (bind _output_get (set `self.redTeamControl` (`KismetMathLibrary.FClamp` (+ (`self.redTeamControl`) (* 2 (`KismetMathLibrary.Conv_IntToDouble` (`KismetMathLibrary.Clamp` (- (`self.numberOfRedOnPoint`) (`self.numberOfBlueOnPoint`)) 1 10)))) 0.0 100.0)))
      (if (> _output_get 24.0)
        (set `self.team` "NewEnumerator0")
        (`MaterialInstanceDynamic.SetVectorParameterValue` (`self.matInst`) "Color" (struct :`R` 0.859375 :`G` 0.044759 :`B` 0.044759 :`A` 1.0))
        (`MaterialInstanceDynamic.SetVectorParameterValue` (`self.matBeamLight`) "Color" (struct :`R` 0.859375 :`G` 0.044759 :`B` 0.044759 :`A` 1.0))
        (`self.updatePlayerStats`)
        (else
          (`self.updatePlayerStats`))))))

(event `updatePlayerStats`
  (bind _asbp_multi_player_game_mode (cast `/Game/MultiplayerStarterPack/Blueprints/BP_MultiPlayerGameMode` (`GameplayStatics.GetGameMode`) :!pure true))
  (`/Engine/EditorBlueprintResources/StandardMacros.IsValid` _asbp_multi_player_game_mode
    (:`Is Valid`
      (`/Game/MultiplayerStarterPack/Blueprints/BP_MultiPlayerGameMode.updateStats` _asbp_multi_player_game_mode))))

(event `clearTimers`
  (`|ExecutionSequence`
    (:`then_0`
      (goto _label_2))
    (:`then_1`
      (goto _label_3))))

(event `blueControlling`
  (bind _redteamcontrol (`self.redTeamControl`))
  (if (> _redteamcontrol 0.0)
    (set `self.redTeamControl` (`KismetMathLibrary.FClamp` (- _redteamcontrol 1.0) 0.0 100.0))
    (else
      (set `self.team` "NewEnumerator2")
      (bind _output_get (set `self.blueTeamControl` (`KismetMathLibrary.FClamp` (+ (`self.blueTeamControl`) (* 2 (`KismetMathLibrary.Conv_IntToDouble` (`KismetMathLibrary.Clamp` (- (`self.numberOfBlueOnPoint`) (`self.numberOfRedOnPoint`)) 1 10)))) 0.0 100.0)))
      (if (> _output_get 24.0)
        (set `self.team` "NewEnumerator1")
        (`MaterialInstanceDynamic.SetVectorParameterValue` (`self.matInst`) "Color" (struct :`R` 0.107422 :`G` 0.284363 :`B` 0.859375 :`A` 1.0))
        (`MaterialInstanceDynamic.SetVectorParameterValue` (`self.matBeamLight`) "Color" (struct :`R` 0.107422 :`G` 0.284363 :`B` 0.859375 :`A` 1.0))
        (`self.updatePlayerStats`)
        (else
          (`self.updatePlayerStats`))))))

(fn `UserConstructionScript`
  (bind _returnvalue (`PrimitiveComponent.CreateDynamicMaterialInstance` (`self.Cone`) 0 "/Game/Materials/Materials/MAT_controlPoint_Inst.MAT_controlPoint_Inst" "None"))
  (set `self.matInst` _returnvalue)
  (bind _returnvalue_2 (`PrimitiveComponent.CreateDynamicMaterialInstance` (`self.Cylinder`) 0 "/Game/Materials/Materials/MAT_oblesikRay_Inst.MAT_oblesikRay_Inst" "None"))
  (set `self.matBeamLight` _returnvalue_2))