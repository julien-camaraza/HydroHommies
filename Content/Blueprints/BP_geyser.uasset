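; Geyser actor that gives multiplayer characters a super jump and refills their water while they stand in its box, with a sound played at BeginPlay.
; Capsule overlap raises jump velocity and air control and starts a looping timer that tops up clamped WaterRemaining on the last character cast.
; End overlap clears the timer and lowers jump velocity at once, then lowers air control after a short delay.
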(event `self.ReceiveBeginPlay`
  (`GameplayStatics.PlaySoundAtLocation` "/Game/Sound/Enviroment/CUE_geyser.CUE_geyser" (`self.K2_GetActorLocation`) (struct) 1.0 1.0 0.0 null null null))

(event `self.Box.OnComponentBeginOverlap`
  (params (OverlappedComponent :type "PrimitiveComponent Object Reference") (OtherActor :type "Actor Object Reference") (OtherComp :type "PrimitiveComponent Object Reference") (OtherBodyIndex :type Integer) (bFromSweep :type Boolean) (SweepResult :type "HitResult Structure (by ref)"))
  (bind _asbp_multiplayer_character (cast `/Game/MultiplayerStarterPack/Blueprints/BP_Multiplayer_Character` OtherActor))
  (if (== OtherComp (`Character.CapsuleComponent` _asbp_multiplayer_character))
    (bind _charactermovement (`Character.CharacterMovement` _asbp_multiplayer_character))
    ;[1 1 1] Super jump
    (set `CharacterMovementComponent.JumpZVelocity` 5000.0 _charactermovement)
    (set `CharacterMovementComponent.AirControl` 1.0 _charactermovement)
    (bind _returnvalue (`KismetSystemLibrary.K2_SetTimerDelegate` (delegate `refillWater`) 0.1 true))))

(event `refillWater`
  (set `/Game/MultiplayerStarterPack/Blueprints/BP_Multiplayer_Character.waterRemaining` (`KismetMathLibrary.FClamp` (+ (`/Game/MultiplayerStarterPack/Blueprints/BP_Multiplayer_Character.waterRemaining` (stale `self.Box.OnComponentBeginOverlap` _asbp_multiplayer_character)) 1.0) 0.0 100.0) (stale `self.Box.OnComponentBeginOverlap` _asbp_multiplayer_character)))

(event `self.Box.OnComponentEndOverlap`
  (params (OverlappedComponent :type "PrimitiveComponent Object Reference") (OtherActor :type "Actor Object Reference") (OtherComp :type "PrimitiveComponent Object Reference") (OtherBodyIndex :type Integer))
  (bind _asbp_multiplayer_character (cast `/Game/MultiplayerStarterPack/Blueprints/BP_Multiplayer_Character` OtherActor))
  (`KismetSystemLibrary.K2_ClearAndInvalidateTimerHandle` (stale `self.Box.OnComponentBeginOverlap` _returnvalue))
  (bind _charactermovement (`Character.CharacterMovement` _asbp_multiplayer_character))
  (set `CharacterMovementComponent.JumpZVelocity` 1500.0 _charactermovement)
  (`KismetSystemLibrary.Delay` 1.5)
  (set `CharacterMovementComponent.AirControl` 0.2 _charactermovement))

(fn `UserConstructionScript`)