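; Game data actor for a Red vs Blue multiplayer round game, tracking team rosters, deaths and round wins.
; Team updates rebuild rosters and start the BP_gameState timer.
; Round end credits the team with more recorded deaths, breaks ties by control points (crediting both if still level), then respawns players and resets timer and HUD scores.
; A separate death check credits wins for team wipes without resetting.
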(event `roundEnd`
  (if (> (`self.redDeaths`) (`self.blueDeaths`))
    (`/Engine/EditorBlueprintResources/StandardMacros.IncrementInt` (`self.redWins`)
      (:`  `
        _))
    (elif (> (`self.blueDeaths`) (`self.redDeaths`))
      (`/Engine/EditorBlueprintResources/StandardMacros.IncrementInt` (`self.blueWins`)
        (:`  `
          _))
      (else
        (for _array_element (`self.controlPoints`)
          (switch `/Game/Blueprints/ENUM_teams` (`/Game/Blueprints/BP_controlPoint.team` _array_element)
            (:`NewEnumerator0`
              (`/Engine/EditorBlueprintResources/StandardMacros.IncrementInt` (`self.controlledRedPoints`)))
            (:`NewEnumerator1`
              (`/Engine/EditorBlueprintResources/StandardMacros.IncrementInt` (`self.controlledBluePoints`)))))
        (if (> (`self.controlledRedPoints`) (`self.controlledBluePoints`))
          (`/Engine/EditorBlueprintResources/StandardMacros.IncrementInt` (`self.redWins`)
            (:`  `
              _))
          (elif (> (`self.controlledBluePoints`) (`self.controlledRedPoints`))
            (`/Engine/EditorBlueprintResources/StandardMacros.IncrementInt` (`self.blueWins`)
              (:`  `
                _))
            (else
              (`/Engine/EditorBlueprintResources/StandardMacros.IncrementInt` (`self.redWins`)
                (:`  `
                  (`/Engine/EditorBlueprintResources/StandardMacros.IncrementInt` (`self.blueWins`)
                    (:`  `
                      _))))))))))
  (`self.resetEverything`))

(event `resetEverything`
  (for _array_element (`self.players`)
    (`/Engine/EditorBlueprintResources/StandardMacros.IsValid` _array_element
      (:`Is Valid`
        (`/Game/MultiplayerStarterPack/Blueprints/BP_Multiplayer_Character.roundRestart` _array_element (`self.redWins`) (`self.blueWins`))
        (`/Game/MultiplayerStarterPack/Blueprints/BP_Multiplayer_Character.respawn` _array_element))))
  (bind _asbp_game_state (cast `/Game/Blueprints/BP_gameState` (`GameplayStatics.GetGameState`))
    (:`then`
      (`/Game/Blueprints/BP_gameState.resetTimer` _asbp_game_state))
    (:`CastFailed`
      _))
  (set `self.redDeaths` 0)
  (set `self.blueDeaths` 0)
  (set `self.controlledBluePoints` 0)
  (set `self.controlledRedPoints` 0)
  (for _array_element_2 (`self.players`)
    (bind _hudwidget (`/Game/MultiplayerStarterPack/Blueprints/BP_Multiplayer_Character.hudWidget` _array_element_2))
    (`/Engine/EditorBlueprintResources/StandardMacros.IsValid` _hudwidget
      (:`Is Valid`
        (`/Game/Widget/BPW_gameHUD.updateScore` _hudwidget (`self.redDeaths`) (`self.blueDeaths`))))))

(event `self.ReceiveBeginPlay`
  (bind _outactors (`GameplayStatics.GetAllActorsOfClass` "/Game/Blueprints/BP_controlPoint.BP_controlPoint_C"))
  (set `self.controlPoints` _outactors)
  (set `self.blueSpawn` (`SceneComponent.K2_GetComponentLocation` (`self.blueSpawnPoint`)))
  (set `self.redSpawn` (`SceneComponent.K2_GetComponentLocation` (`self.redSpawnPoint`))))

(event `updateScore`
  (params (deadPlayersTeam :type "/Game/Blueprints/ENUM_teams Enum" :default "NewEnumerator2"))
  (switch `/Game/Blueprints/ENUM_teams` deadPlayersTeam
    (:`NewEnumerator0`
      (`/Engine/EditorBlueprintResources/StandardMacros.IncrementInt` (`self.redDeaths`)
        (:`  `
          _)))
    (:`NewEnumerator1`
      (`/Engine/EditorBlueprintResources/StandardMacros.IncrementInt` (`self.blueDeaths`)
        (:`  `
          _))))
  (for _array_element (`self.players`)
    (bind _hudwidget (`/Game/MultiplayerStarterPack/Blueprints/BP_Multiplayer_Character.hudWidget` _array_element)
      (:`then`
        (`/Game/Widget/BPW_gameHUD.updateScore` _hudwidget (`self.redDeaths`) (`self.blueDeaths`)))
      (:`else`))))

(event `checkDeath`
  (bind _blueteam (`self.blueTeam`))
  ;[1 1 1] When players die, check if all of them on one team are dead
  (set `self.deadBluePeople` 0)
  (set `self.deadRedPeople` 0)
  (for _array_element _blueteam
    (if (`/Game/MultiplayerStarterPack/Blueprints/BP_Multiplayer_Character.Dead` _array_element)
      (`/Engine/EditorBlueprintResources/StandardMacros.IncrementInt` (`self.deadBluePeople`))))
  (if (== (`self.deadBluePeople`) (`KismetArrayLibrary.Array_Length` _blueteam))
    (`/Engine/EditorBlueprintResources/StandardMacros.IncrementInt` (`self.redWins`))
    (else
      (for _array_element_2 (`self.redTeam`)
        (if (`/Game/MultiplayerStarterPack/Blueprints/BP_Multiplayer_Character.Dead` _array_element_2)
          (`/Engine/EditorBlueprintResources/StandardMacros.IncrementInt` (`self.deadRedPeople`))))
      (if (== (`self.deadRedPeople`) (`KismetArrayLibrary.Array_Length` (`self.redTeam`)))
        (`/Engine/EditorBlueprintResources/StandardMacros.IncrementInt` (`self.blueWins`))))))

(event `SR_updateTeams`
  (`KismetArrayLibrary.Array_Clear` (`self.readyPlayers`))
  (`KismetArrayLibrary.Array_Clear` (`self.redTeam`))
  (`KismetArrayLibrary.Array_Clear` (`self.blueTeam`))
  (`KismetArrayLibrary.Array_Clear` (`self.players`))
  (bind _outactors (`GameplayStatics.GetAllActorsOfClass` "/Game/MultiplayerStarterPack/Blueprints/BP_Multiplayer_Character.BP_Multiplayer_Character_C"))
  (for _array_element _outactors
    (`KismetArrayLibrary.Array_AddUnique` (`self.players`) _array_element)
    (`KismetArrayLibrary.Array_Add` (`self.readyPlayers`))
    (switch `/Game/Blueprints/ENUM_teams` (`/Game/MultiplayerStarterPack/Blueprints/BP_Multiplayer_Character.team` _array_element)
      (:`NewEnumerator0`
        (`KismetArrayLibrary.Array_AddUnique` (`self.redTeam`) _array_element))
      (:`NewEnumerator1`
        (`KismetArrayLibrary.Array_AddUnique` (`self.blueTeam`) _array_element))))
  (set `self.minutesRemaining` 2)
  (set `self.secondsRemaining` 0)
  (bind _asbp_game_state (cast `/Game/Blueprints/BP_gameState` (`GameplayStatics.GetGameState`)))
  (`/Game/Blueprints/BP_gameState.startTimer` _asbp_game_state))

(event `unreadyPlayers`
  (bind _readyplayers (`self.readyPlayers`))
  (for (_ _array_index) _readyplayers
    (`KismetArrayLibrary.Array_Set` _readyplayers _array_index)))

(event `respawnPlayers`
  (for _array_element (`self.players`)
    (`/Game/MultiplayerStarterPack/Blueprints/BP_Multiplayer_Character.respawn` _array_element)))

(event `timer`
  (bind _result (`/Engine/EditorBlueprintResources/StandardMacros.DecrementInt` (`self.secondsRemaining`))
    (:`  `
      (if (< _result 0)
        (if (< (`self.minutesRemaining`) 1)
          (`self.roundEnd`)
          (else
            (set `self.secondsRemaining` 59)
            (`/Engine/EditorBlueprintResources/StandardMacros.DecrementInt` (`self.minutesRemaining`))))))))

(fn `UserConstructionScript`)