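; Multiplayer game mode for Red versus Blue control-point play, rewarding each team for the points it holds.
; On BeginPlay it caches all control points, and updateWidget adds one hill tracker bar per point to the HUD.
; updateStats counts points per team and scales that team's members' damage and speed multipliers linearly with the count.
; Team updating, timer restart and round end are empty stubs.
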(event `updateWidget`
  (params (hudWidget :type "/Game/Widget/BPW_gameHUD Object Reference"))
  ;[1 1 1] Adds a bar to the widget for each control point
  (for _ (`self.controlPoints`)
    (bind _returnvalue (`|CreateWidget` "/Game/Widget/BPW_hillTracker.BPW_hillTracker_C"))
    (`PanelWidget.AddChild` (`/Game/Widget/BPW_gameHUD.VerticalBox_0` hudWidget) _returnvalue)))

(event `self.ReceiveBeginPlay`
  (bind _outactors (`GameplayStatics.GetAllActorsOfClass` "/Game/Blueprints/BP_controlPoint.BP_controlPoint_C"))
  (set `self.controlPoints` _outactors))

(event `updateTeams`)

(event `updateStats`
  (set `self.controlledRedPoints` 0)
  (set `self.controlledBluePoints` 0)
  (for _array_element (`self.controlPoints`)
    (switch `/Game/Blueprints/ENUM_teams` (`/Game/Blueprints/BP_controlPoint.team` _array_element)
      (:`NewEnumerator0`
        (`/Engine/EditorBlueprintResources/StandardMacros.IncrementInt` (`self.controlledRedPoints`)))
      (:`NewEnumerator1`
        (`/Engine/EditorBlueprintResources/StandardMacros.IncrementInt` (`self.controlledBluePoints`)))))
  (`|ExecutionSequence`
    (:`then_0`
      (for _array_element_2 (`self.redTeam`)
        (set `/Game/MultiplayerStarterPack/Blueprints/BP_Multiplayer_Character.damageMultiplier` (+ (* (`self.controlledRedPoints`) 0.25) 0.25) _array_element_2)
        (set `/Game/MultiplayerStarterPack/Blueprints/BP_Multiplayer_Character.speedMultiplier` (+ (* (`self.controlledRedPoints`) 0.25) 1.0) _array_element_2)))
    (:`then_1`
      (for _array_element_3 (`self.blueTeam`)
        (set `/Game/MultiplayerStarterPack/Blueprints/BP_Multiplayer_Character.damageMultiplier` (+ (* (`self.controlledBluePoints`) 0.25) 0.25) _array_element_3)
        (set `/Game/MultiplayerStarterPack/Blueprints/BP_Multiplayer_Character.speedMultiplier` (+ (* (`self.controlledBluePoints`) 0.25) 1.0) _array_element_3)))))

(event `restartTimer`)

(fn `roundEnd`)

(fn `UserConstructionScript`)