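; Game instance Blueprint for multiplayer that handles hosting, joining and leaving sessions through three custom events.
; Hosting creates a session with the given connection count and LAN flag, then opens the AncientWatersMapFlatWalk map as a listen server.
; Hosting and joining switch the player to game-only input with a hidden cursor, while leaving destroys the session and opens the Lobby level.
; Each success or failure only prints a message besides these actions.
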(event `HOST_SESSION`
  (params (PublicConnections :type Integer) (bUseLAN :type Boolean))
  (bind _returnvalue (`GameplayStatics.GetPlayerController` 0))
  ;[1 1 1] HostSession
  (`CreateSessionCallbackProxy.CreateSession` (`GameplayStatics.GetPlayerController` 0) PublicConnections bUseLAN
    (:`OnSuccess`
      (`KismetSystemLibrary.PrintString` "Session Created")
      (`WidgetBlueprintLibrary.SetInputMode_GameOnly` _returnvalue)
      (set `PlayerController.bShowMouseCursor` false _returnvalue)
      (`GameplayStatics.OpenLevel` "AncientWatersMapFlatWalk" true "listen"))
    (:`OnFailure`
      (`KismetSystemLibrary.PrintString` "Could not create a session"))))

(event `JOIN_SESSION`
  (params (SessionToJoin :type "BlueprintSessionResult Structure (by ref)"))
  (bind _returnvalue (`GameplayStatics.GetPlayerController` 0))
  ;[1 1 1] joinSession
  (`JoinSessionCallbackProxy.JoinSession` (`GameplayStatics.GetPlayerController` 0) SessionToJoin
    (:`OnSuccess`
      (`KismetSystemLibrary.PrintString` "Session Joined")
      (`WidgetBlueprintLibrary.SetInputMode_GameOnly` _returnvalue)
      (set `PlayerController.bShowMouseCursor` false _returnvalue))
    (:`OnFailure`
      (`KismetSystemLibrary.PrintString` "Could not join a session"))))

(event `DestroySession`
  (params (PlayerController :type "PlayerController Object Reference"))
  ;[1 1 1] DestroySession
  (`DestroySessionCallbackProxy.DestroySession` PlayerController
    (:`OnSuccess`
      (`KismetSystemLibrary.PrintString` "SessionLeft")
      (`GameplayStatics.OpenLevel` "Lobby"))
    (:`OnFailure`
      (`KismetSystemLibrary.PrintString` "Error"))))